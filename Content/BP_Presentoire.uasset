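; A display stand actor that shows an item for sale and registers itself with the player character when nearby.
; A slowed timeline spins the widget component around its yaw axis.
; MiseEnVente writes the item's enum name and price into the cached Wid_Presentoire widget.
; Box overlaps toggle the TopDownCharacter's range state through InRagneSwitch and set or clear its PresRef to this stand.
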(event OnComponentBeginOverlap(Box)
  (params (OverlappedComponent :type Primitive%20Component%20Object%20Reference) (OtherActor :type Actor%20Object%20Reference) (OtherComp :type Primitive%20Component%20Object%20Reference) (OtherBodyIndex :type Integer) (bFromSweep :type Boolean) (SweepResult :type Hit%20Result%20Structure%20%28by%20ref%29))
  (bind _astop_down_character (Utilities|Casting|CastToTopDownCharacter OtherActor))
  (Default|InRagneSwitch _astop_down_character)
  (Variables|/Game/TopDownBP/Blueprints/TopDownCharacter.TopDownCharacter_C|SetPresRef _astop_down_character self))

(event OnComponentEndOverlap(Box)
  (params (OverlappedComponent :type Primitive%20Component%20Object%20Reference) (OtherActor :type Actor%20Object%20Reference) (OtherComp :type Primitive%20Component%20Object%20Reference) (OtherBodyIndex :type Integer))
  (bind _astop_down_character (Utilities|Casting|CastToTopDownCharacter OtherActor))
  (Default|InRagneSwitch _astop_down_character)
  (Variables|/Game/TopDownBP/Blueprints/TopDownCharacter.TopDownCharacter_C|SetPresRef _astop_down_character 0))

(event Custom|MiseEnVente
  (params (Mise%20En%20Vente :type Struct%20Article%20En%20Vente%20Structure))
  (bind _wid_presentoire (Variables|Default|GetWid_Presentoire))
  (Rendering|Components|TextRender|SetText (Variables|/Game/Wid_Presentoire.Wid_Presentoire_C|GetNom _wid_presentoire) (Utilities|Text|ToText(String) (Utilities|String|EnumtoString (.nom Mise%20En%20Vente))))
  (Rendering|Components|TextRender|SetText (Variables|/Game/Wid_Presentoire.Wid_Presentoire_C|GetPrix _wid_presentoire) (Utilities|Text|ToText(Integer) (.prix Mise%20En%20Vente))))

(event EventBeginPlay
  (Utilities|FlowControl|Sequence
    (:then_0
      (Components|Timeline|SetPlayRate (Variables|Default|GetRotateWid) 0.1)
      (bind _newtrack_0 (Timeline|RotateWid Play)
        (:Update
          (Transformation|SetRelativeRotation (Variables|Default|GetWidget) (Math|Rotator|MakeRotator 0.0 0.0 (* _newtrack_0 3.6e+02)) false false))))
    (:then_1
      (bind _aswid_presentoire (Utilities|Casting|CastToWid_Presentoire (UserInterface|GetWidget (Variables|Default|GetWidget))))
      (Variables|Default|SetWid_Presentoire _aswid_presentoire))))

(fn ConstructionScript)